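; Runtime transform gizmo that, on BeginPlay, copies the GizmoPlayerController's selected actors as its targets, if any exist.
; ClientMoveActor forwards a location and target to ServerMoveActor, which sets that actor's location without sweep.
; Tick is empty, and nothing in this Blueprint calls the move chain from a live path.
; Unconnected leftover nodes would toggle a dynamic-material highlight and send the first target's current location to ServerMoveActor.
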(event Custom|ClientMoveActor
  (params (NewParam :type Vector) (Target :type Actor%20Object%20Reference))
  (CallFunction|ServerMOveActor NewParam Target))

(event Custom|ServerMoveActor
  (params (NewParam :type Vector) (Target :type Actor%20Object%20Reference))
  (Transformation|SetActorLocation Target NewParam false false))

(event EventBeginPlay
  (bind _asgizmo_player_controller (Utilities|Casting|CastToGizmoPlayerController (Game|GetPlayerController 0)))
  (if (> (Utilities|Array|Length (Variables|/Script/Gizmo.GizmoPlayerController|GetSelectedActors _asgizmo_player_controller)) 0)
    (Variables|Default|SetTargetActor (Variables|/Script/Gizmo.GizmoPlayerController|GetSelectedActors _asgizmo_player_controller))))

(event EventEndPlay
  (params (EndPlayReason :type EEndPlayReason%20Enum :default "Destroyed")))

(event EventTick
  (params (DeltaSeconds :type Float%20%28single-precision%29)))

(fn ConstructionScript)